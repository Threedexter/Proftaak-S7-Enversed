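; Pickup actor that comes in Gold, Silver or Bronze types and carries a score value.
; The construction script sets the Pickup component's material from its type.
; On overlap it asks the other actor whether it can pick up and, if so, passes itself to that actor's PickupMessage.
; Getters expose score and type, though GetPickupType always returns Gold, CanPickup always returns true and SetPlayerCanPickup is empty.
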(event `self.Pickup.OnComponentBeginOverlap`
  (params (OverlappedComponent :type "PrimitiveComponent Object Reference") (OtherActor :type "Actor Object Reference") (OtherComp :type "PrimitiveComponent Object Reference") (OtherBodyIndex :type Integer) (bFromSweep :type Boolean) (SweepResult :type "HitResult Structure (by ref)"))
  ;[1 1 1] Basic pickup mechanic
  (bind _canpickup (message `/Game/Blueprints/Pawns/Interfaces/IPawn.CanPickup` OtherActor))
  (if _canpickup
    (message `/Game/Blueprints/Pawns/Interfaces/IPawn.Pickup` OtherActor self)))

(fn `CanPickup`
  (returns (CanPickup :type Boolean))
  (return true))

(fn `GetPickupScore`
  (returns (Score :type Integer))
  (return (`self.PickupScore`)))

(fn `GetPickupType`
  (returns (Type :type "/Game/Blueprints/Pickup/Enums/EPickupType Enum"))
  (return "NewEnumerator0"))

(fn `SetPlayerCanPickup`
  (params (CanPickup :type Boolean)))

(fn `UserConstructionScript`
  (`PrimitiveComponent.SetMaterial` (`self.Pickup`) 0 (select `/Game/Blueprints/Pickup/Enums/EPickupType` (`self.PickupType`) :`NewEnumerator0` (`self.MaterialGold`) :`NewEnumerator1` (`self.MaterialSilver`) :`NewEnumerator2` (`self.MaterialBronze`))))