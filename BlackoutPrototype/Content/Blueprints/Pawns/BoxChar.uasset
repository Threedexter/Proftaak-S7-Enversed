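; BoxChar is a player-controlled pawn with basic axis movement and a respawn event.
; MoveForward and MoveRight inputs feed movement along the capsule's forward and right vectors.
; Respawn sends the controller and the pawn itself to the game mode through SpawnMessage, then detaches the controller and destroys the actor.
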(event `InputAxis|MoveForward`
  (params (AxisValue :type "Float (single-precision)"))
  ;[1 1 1] Movement
  (`self.AddMovementInput` (`SceneComponent.GetForwardVector` (`self.CapsuleComponent`)) AxisValue))

(event `InputAxis|MoveRight`
  (params (AxisValue :type "Float (single-precision)"))
  ;[1 1 1] Movement
  (`self.AddMovementInput` (`SceneComponent.GetRightVector` (`self.CapsuleComponent`)) AxisValue))

(event `/Game/Blueprints/Pawns/Interfaces/IPawn.Respawn`
  ;[1 1 1] Simple respawn event
  (message `/Game/Blueprints/GM/Interfaces/IGameMode.Spawn` (`GameplayStatics.GetGameMode`) (`self.GetController`) self)
  (`self.DetachFromControllerPendingDestroy`)
  (`self.K2_DestroyActor`))

(fn `UserConstructionScript`)