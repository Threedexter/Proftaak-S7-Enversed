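; BlackoutGameMode is the game mode that handles spawning, pawn choice and HUD setup for split-screen players.
; GetSpawnpoint picks a random SpawnPoint that reports it can spawn, falling back to any, and feeds both ChoosePlayerStart and Spawn.
; Spawn creates the given class there and has the supplied player or AI controller possess it.
; Player controller ID 0 gets the default pawn and first-person HUD, while other players get alternate ones.
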(event `self.InitSpawnPoints`
  ;[1 1 1] Gets all the spawnpoints
  (bind _outactors (`GameplayStatics.GetAllActorsOfClass` "/Game/Blueprints/Spawn/SpawnPoint.SpawnPoint_C"))
  (set `self.SpawnPoints` _outactors))

(event `self.Spawn`
  (params (Controller :type "Controller Object Reference") (Type :type "Object Object Reference"))
  ;[1 1 1] Respawn AI or Player
  (set `self.RespawnController` Controller)
  (bind _spawnpoint (`self.GetSpawnpoint`))
  (message `/Game/Blueprints/Spawn/Interfaces/SpawnInterface.SetSpawned` _spawnpoint)
  (bind _asactor (castclass `Actor` (`GameplayStatics.GetObjectClass` Type))
    (:`then`
      (bind _spawnpoint_2 (message `/Game/Blueprints/Spawn/Interfaces/SpawnInterface.GetSpawnPoint` _spawnpoint))
      (bind _returnvalue (`|SpawnActorFromClass` _asactor (`KismetMathLibrary.MakeTransform` (.location _spawnpoint_2) (.rotation _spawnpoint_2)) "Undefined" "OverrideRootScale" null null))
      (bind _aspawn (cast `Pawn` _returnvalue)
        (:`then`
          _)
        (:`CastFailed`
          _))
      (`Controller.Possess` (`self.RespawnController`) _aspawn))
    (:`CastFailed`
      (`KismetSystemLibrary.PrintString` "FailedToSpawn"))))

(event `self.InitializeHUDForPlayer`
  (params (NewPlayer :type "PlayerController Object Reference"))
  ;[1 1 1] Setup the right HUDS for the player
  (bind _returnvalue (`GameplayStatics.GetPlayerControllerID` NewPlayer))
  (if (== _returnvalue 0)
    (`PlayerController.ClientSetHUD` NewPlayer "/Game/FirstPersonBP/Blueprints/FirstPersonHUD.FirstPersonHUD_C")
    (else
      (`PlayerController.ClientSetHUD` NewPlayer "/Game/Blueprints/UI/BoxPlayerHUD.BoxPlayerHUD_C"))))

(fn `ChoosePlayerStart`
  (params (Player :type "Controller Object Reference"))
  (returns (ReturnValue :type "Actor Object Reference"))
  (bind _spawnpoint (`self.GetSpawnpoint`))
  (`/Engine/EditorBlueprintResources/StandardMacros.IsValid` _spawnpoint
    (:`Is Valid`
      (message `/Game/Blueprints/Spawn/Interfaces/SpawnInterface.SetSpawned` _spawnpoint)
      (return _spawnpoint))
    (:`Is Not Valid`
      (`KismetSystemLibrary.PrintString` "Couldnt get the spawnpoint"))))

(fn `GetDefaultPawnClassForController`
  (params (InController :type "Controller Object Reference"))
  (returns (ReturnValue :type "Object Class Reference"))
  (bind _asplayer_controller (cast `PlayerController` InController)
    (:`then`
      (bind _returnvalue (`GameplayStatics.GetPlayerControllerID` _asplayer_controller))
      (if (== _returnvalue 0)
        (return (`self.DefaultPawnClass`))
        (else
          (return (`self.OtherSplitScreenActor`)))))
    (:`CastFailed`
      (return (`self.DefaultPawnClass`)))))

(fn `GetSpawnpoint`
  (returns (SpawnPoint :type "Actor Object Reference"))
  (locals (AvailableSpawnPoints :type "Array of Actor Object Reference"))
  (bind _spawnpoints (`self.SpawnPoints`))
  (bind _availablespawnpoints (`local.AvailableSpawnPoints`))
  (bind _returnvalue (`KismetArrayLibrary.Array_Length` _spawnpoints))
  (bind _returnvalue_2 (`KismetArrayLibrary.Array_Length` _availablespawnpoints))
  (if (not (> _returnvalue 0))
    (`self.InitSpawnPoints`))
  (for _array_element _spawnpoints
    (bind _spawnable (message `/Game/Blueprints/Spawn/Interfaces/SpawnInterface.CanSpawn` _array_element))
    (if _spawnable
      (`KismetArrayLibrary.Array_Add` (`local.AvailableSpawnPoints`) _array_element)))
  (if (> _returnvalue_2 0)
    (return (`|GetArrayItem` _availablespawnpoints (`KismetMathLibrary.RandomIntegerInRange` 0 (- _returnvalue_2 1))))
    (else
      (return (`|GetArrayItem` _spawnpoints (`KismetMathLibrary.RandomIntegerInRange` 0 (- _returnvalue 1)))))))

(fn `UserConstructionScript`)