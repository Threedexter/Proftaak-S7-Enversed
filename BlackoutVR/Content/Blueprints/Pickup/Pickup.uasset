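; Pickup actor with a Gold, Silver or Bronze type and a score value, collected when an actor overlaps its Pickup component.
; On overlap it asks the other actor whether it can pick up, then passes itself via PickupMessage.
; The construction script sets the component's material from PickupType.
; Getters expose the score, but GetPickupType always returns Gold, CanPickup always returns true, and SetPlayerCanPickup is empty.
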(event `self.ReceiveBeginPlay`)

(event `self.Pickup.OnComponentBeginOverlap`
  (params (OverlappedComponent :type "PrimitiveComponent Object Reference") (OtherActor :type "Actor Object Reference") (OtherComp :type "PrimitiveComponent Object Reference") (OtherBodyIndex :type Integer) (bFromSweep :type Boolean) (SweepResult :type "HitResult Structure (by ref)"))
  ;[1 1 1] Basic pickup mechanic
  (bind _canpickup (message `/Game/Blueprints/Pickup/Interfaces/IPickup.CanPickup` OtherActor))
  (if _canpickup
    (message `/Game/Blueprints/Pickup/Interfaces/IScore.Pickup` OtherActor self)))

(event `InputTouch`
  (params (Location :type "Vector Structure") (FingerIndex :type "ETouchIndex Enum")))

(fn `CanPickup`
  (returns (CanPickup :type Boolean))
  (return true))

(fn `GetPickupScore`
  (returns (Score :type Integer))
  (return (`self.PickupScore`)))

(fn `GetPickupType`
  (returns (Type :type "/Game/Blueprints/Pickup/Enums/EPickupType Enum"))
  (return "NewEnumerator0"))

(fn `SetPlayerCanPickup`
  (params (CanPickup :type Boolean)))

(fn `UserConstructionScript`
  (bind _pickup (`self.Pickup`))
  (bind _returnvalue (select `/Game/Blueprints/Pickup/Enums/EPickupType` (`self.PickupType`) :`NewEnumerator0` (`self.MaterialGold`) :`NewEnumerator1` (`self.MaterialSilver`) :`NewEnumerator2` (`self.MaterialBronze`)))
  (if (and (`KismetSystemLibrary.IsValid` _returnvalue) (`KismetSystemLibrary.IsValid` _pickup))
    (`PrimitiveComponent.SetMaterial` _pickup 0 _returnvalue)))