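; Touch-controlled actor that takes damage, collects pickups for score and can itself be picked up but not dropped.
; Damage awards points to the instigator's pawn, with a larger bonus on a kill, when the game mode is asked to respawn the actor.
; At BeginPlay it caches the SpectatorUI from a MySpectorCapture actor's widget, then sends it touch start/end events by TouchActorID as movement starts and stops.
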(event `self.ReceiveBeginPlay`
  (`self.setSpectatorUI`))

(event `self.ReceiveAnyDamage`
  (params (Damage :type "Float (single-precision)") (DamageType :type "DamageType Object Reference") (InstigatedBy :type "Controller Object Reference") (DamageCauser :type "Actor Object Reference"))
  (bind _returnvalue (`Controller.K2_GetPawn` InstigatedBy))
  ;[1 1 1] Damage event
  (bind _output_get (set `self.Health` (- (`self.Health`) Damage)))
  (if (< _output_get 0.5)
    (`/Game/Blueprints/Pickup/Interfaces/ITouch.Respawn`)
    (message `ScoreKeeper.AddToScore` _returnvalue 250)
    (else
      (message `ScoreKeeper.AddToScore` _returnvalue 100))))

(event `/Game/Blueprints/Pickup/Interfaces/ITouch.Respawn`
  ;[1 1 1] Respawn logic
  (message `/Game/Blueprints/GameMode/Interfaces/IBlackoutGM.RespawnTouchActor` (`GameplayStatics.GetGameMode`) self))

(event `/Game/Blueprints/Pickup/Interfaces/ITouch.Pickup`
  (params (`Object To Pickup` :type "Actor Object Reference"))
  ;[1 1 1] Pickup Event
  (bind _score (message `/Game/Blueprints/Pickup/Interfaces/IPickup.GetPickupScore` `Object To Pickup`))
  (`ScoreKeeper.AddToScore` _score)
  (`self.K2_DestroyActor` `Object To Pickup`)
  (bind _returnvalue (`ScoreKeeper.GetScore`))
  (`KismetSystemLibrary.PrintString` (`KismetStringLibrary.Concat_StrStr` (`KismetSystemLibrary.GetObjectName` self) "-" (`KismetStringLibrary.Conv_IntToString` _returnvalue))))

(event `self.ActorStoppedMoving`
  (`/Game/Art/UI/SpectatorUI.TouchEndDispatcher_Event` (`self.SpectatorUI`) (`self.TouchActorID`)))

(event `self.ActorStartedMoving`
  (`/Game/Art/UI/SpectatorUI.TouchStartDispatcher_Event` (`self.SpectatorUI`) (`self.TouchActorID`)))

(fn `CanDrop`
  (returns (`Can Drop` :type Boolean))
  (return false))

(fn `CanPickup`
  (returns (`Can Pickup` :type Boolean))
  (return true))

(fn `GetCName`
  (returns (ReturnValue :type String))
  (return (`self.Name`)))

(fn `UserConstructionScript`)