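; Pressure pad that becomes active while touch players stand on it and reports when it is pressed and released.
; Box overlap events count actors implementing TouchActor and keep a list of ExampleTouchPlayerPawns, exposed through GetPlayers.
; The count gates the active flag and enter/exit trigger calls, intended for first arrival and last departure.
; The count changes before the pawn cast, so other TouchActor implementers also affect it.
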(event `self.ReceiveTick`
  (params (DeltaSeconds :type "Float (single-precision)")))

(event `self.Box.OnComponentBeginOverlap`
  (params (OverlappedComponent :type "PrimitiveComponent Object Reference") (OtherActor :type "Actor Object Reference") (OtherComp :type "PrimitiveComponent Object Reference") (OtherBodyIndex :type Integer) (bFromSweep :type Boolean) (SweepResult :type "HitResult Structure (by ref)"))
  (if (`KismetSystemLibrary.DoesImplementInterface` OtherActor "/Script/BlackoutVR.TouchActor")
    (bind _result (`/Engine/EditorBlueprintResources/StandardMacros.IncrementInt` (`self.AmtPlayersOnPad`))
      (:`  `
        (bind _asexample_touch_player_pawn (cast `/EnversedTouch/Example/PlayerPawns/ExampleTouchPlayerPawn` OtherActor))
        (`KismetArrayLibrary.Array_AddUnique` (`self.Players`) _asexample_touch_player_pawn)
        (if (<= _result 1)
          (`self.OnPlayerEnterTrigger`)
          (set `self.IsActive` true))))))

(event `self.Box.OnComponentEndOverlap`
  (params (OverlappedComponent :type "PrimitiveComponent Object Reference") (OtherActor :type "Actor Object Reference") (OtherComp :type "PrimitiveComponent Object Reference") (OtherBodyIndex :type Integer))
  (if (`KismetSystemLibrary.DoesImplementInterface` OtherActor "/Script/BlackoutVR.TouchActor")
    (bind _result (`/Engine/EditorBlueprintResources/StandardMacros.DecrementInt` (`self.AmtPlayersOnPad`))
      (:`  `
        (bind _asexample_touch_player_pawn (cast `/EnversedTouch/Example/PlayerPawns/ExampleTouchPlayerPawn` OtherActor))
        (`KismetArrayLibrary.Array_RemoveItem` (`self.Players`) _asexample_touch_player_pawn)
        (if (<= _result 0)
          (`self.OnPlayerExitTrigger`)
          (set `self.IsActive` false))))))

(fn `GetPlayers`
  (returns (Players :type "Array of /EnversedTouch/Example/PlayerPawns/ExampleTouchPlayerPawn Object Reference"))
  (return (`self.Players`)))

(fn `UserConstructionScript`)