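; BP_Cable is a cable actor that visually shows a Being Captured, Active or Disabled state.
; On BeginPlay it binds itself to every BP_Server whose ID appears in ServersToBindTo.
; Its SetMaterial event acts only on state changes, swapping the material and custom depth stencil value on the mesh and both connection points.
; The construction script toggles each connection point's visibility, while leftover mesh-spawning logic never runs.
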(event `self.ReceiveBeginPlay`
  (bind _outactors (`GameplayStatics.GetAllActorsOfClass` "/Game/Blueprints/Objects/BP_Server.BP_Server_C"))
  (bind _output_get (set `self.PhaseServers` _outactors))
  (for _array_element _output_get
    (for _array_element_2 (`self.ServersToBindTo`)
      (if (== _array_element_2 (`/Game/Blueprints/Objects/BP_Server.ID` _array_element))
        (`/Game/Blueprints/Objects/BP_Server.Bind` _array_element self)))))

(event `/Game/Blueprints/Objects/ServerCableInterface.SetMaterial`
  (params (CableState :type "/Game/Blueprints/Objects/EServerCable Enum" :default "NewEnumerator2"))
  (if (not (== CableState (`self.CurrentState`)))
    (bind _output_get (set `self.CurrentState` CableState))
    (switch `/Game/Blueprints/Objects/EServerCable` _output_get
      (:`NewEnumerator2`
        (`PrimitiveComponent.SetMaterial` (`self.StaticMesh`) 0 (`self.CaptureMaterial`))
        (`PrimitiveComponent.SetMaterial` (`self.ConnectPointRight`) 0 (`self.CaptureMaterial`))
        (`PrimitiveComponent.SetMaterial` (`self.ConnectPointLeft`) 0 (`self.CaptureMaterial`))
        (`PrimitiveComponent.SetCustomDepthStencilValue` (`self.ConnectPointLeft`) 255)
        (`PrimitiveComponent.SetCustomDepthStencilValue` (`self.StaticMesh`) 255)
        (`PrimitiveComponent.SetCustomDepthStencilValue` (`self.ConnectPointRight`) 255))
      (:`NewEnumerator1`
        (`PrimitiveComponent.SetMaterial` (`self.StaticMesh`) 0 (`self.ActiveMaterial`))
        (`PrimitiveComponent.SetMaterial` (`self.ConnectPointRight`) 0 (`self.ActiveMaterial`))
        (`PrimitiveComponent.SetMaterial` (`self.ConnectPointLeft`) 0 (`self.ActiveMaterial`))
        (`PrimitiveComponent.SetCustomDepthStencilValue` (`self.ConnectPointLeft`) 128)
        (`PrimitiveComponent.SetCustomDepthStencilValue` (`self.StaticMesh`) 128)
        (`PrimitiveComponent.SetCustomDepthStencilValue` (`self.ConnectPointRight`) 128))
      (:`NewEnumerator0`
        (`PrimitiveComponent.SetMaterial` (`self.StaticMesh`) 0 (`self.DisabledMaterial`))
        (`PrimitiveComponent.SetMaterial` (`self.ConnectPointRight`) 0 (`self.DisabledMaterial`))
        (`PrimitiveComponent.SetMaterial` (`self.ConnectPointLeft`) 0 (`self.DisabledMaterial`))
        (`PrimitiveComponent.SetCustomDepthStencilValue` (`self.ConnectPointLeft`) 0)
        (`PrimitiveComponent.SetCustomDepthStencilValue` (`self.StaticMesh`) 0)
        (`PrimitiveComponent.SetCustomDepthStencilValue` (`self.ConnectPointRight`) 0)))))

(fn `UserConstructionScript`
  (locals (Servers :type "Array of /Game/Blueprints/Objects/BP_Server Object Reference"))
  (bind _connectpointleft (`self.ConnectPointLeft`))
  (bind _connectpointright (`self.ConnectPointRight`))
  (`|ExecutionSequence`
    (:`then_0`
      (if (`self.HasConnectionRight`)
        (`SceneComponent.SetVisibility` _connectpointright true false)
        (else
          (`SceneComponent.SetVisibility` _connectpointright false false))))
    (:`then_1`
      (if (`self.HasConnectionLeft`)
        (`SceneComponent.SetVisibility` _connectpointleft true false)
        (else
          (`SceneComponent.SetVisibility` _connectpointleft false false))))))