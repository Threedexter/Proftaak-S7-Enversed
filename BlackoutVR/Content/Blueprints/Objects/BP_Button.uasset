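; BP_Button is a physical pressable button that slides Cube2 between its start and maximum positions, raising empty press, fully-pressed and release events.
; Each tick it either follows a line trace hit or, without tracing, pushes while extra components overlap Cube2.
; In overlap mode, it eases back once the ButtonPredictor volume is also clear.
; Any damage also pushes it, and it reports an interactable type.
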(event `self.ReceiveBeginPlay`
  (bind _location (`self.SetDefaultButtonlocation`))
  (`self.SetMaxbuttonLocation` _location)
  (set `self.ButtonComponentAmount` (`KismetArrayLibrary.Array_Length` (`PrimitiveComponent.GetOverlappingComponents` (`self.Cube2`)))))

(event `Button Fully Pressed`)

(event `Button Press`)

(event `Button Release`)

(event `self.ReceiveAnyDamage`
  (params (Damage :type "Float (single-precision)") (DamageType :type "DamageType Object Reference") (InstigatedBy :type "Controller Object Reference") (DamageCauser :type "Actor Object Reference"))
  (`self.PushButton` 100.0))

(event `self.ReceiveTick`
  (params (DeltaSeconds :type "Float (single-precision)"))
  (bind (_start _end _upvector) (`self.GetRangeUp` (`self.Cube2`) (`self.Button range`)))
  (if (`self.UseTrace`)
    (bind (_outhit _returnvalue) (`KismetSystemLibrary.LineTraceSingle` _start _end "TraceTypeQuery1"))
    (`self.MoveButton` _returnvalue (`self.CalculateOffset` _upvector) (`.Location` (`GameplayStatics.BreakHitResult` _outhit)))
    (elif (`self.HasOverlapOnButton`)
      (`self.PushButton` 0.5)
      (elif (not (`self.WillOverlapButton`))
        (`self.ReleaseButton`)))))

(fn `HasGameStarted`
  (returns (Started :type Boolean))
  (bind _started (message `/Game/Blueprints/GameMode/Interfaces/IBlackoutGM.HasGameStarted` (`GameplayStatics.GetGameMode`)))
  (return _started))

(fn `MoveButton`
  (params (HitResult :type Boolean) (MovementVector :type "Vector Structure") (HitVector :type "Vector Structure"))
  (bind _returnvalue (+ HitVector MovementVector))
  (bind _cube2 (`self.Cube2`))
  (if HitResult
    (if (`self.Exceeds` (`self.Max Button Location`) _returnvalue)
      (`SceneComponent.K2_SetWorldLocation` _cube2 (`self.Max Button Location`) false false)
      (if (not (`self.FullyPressed`))
        (set `self.FullyPressed` true)
        (`self.Button Fully Pressed`))
      (if (not (`self.Pressed`)) :!label _label
        (set `self.Pressed` true)
        (`self.Button Press`))
      (elif (`self.Exceeds` _returnvalue (`self.Default Button location`))
        (`SceneComponent.K2_SetWorldLocation` _cube2 (`self.Default Button location`) false false :!label _label_2)
        (if (`self.Pressed`)
          (set `self.Pressed` false)
          (set `self.FullyPressed` false)
          (`self.Button Release`))
        (else
          (`SceneComponent.K2_SetWorldLocation` _cube2 _returnvalue false false)
          (set `self.FullyPressed` false)
          (goto _label))))
    (else
      (goto _label_2))))

(fn `PushButton`
  (params (Distance :type "Float (double-precision)"))
  (locals (NewLoc :type "Vector Structure"))
  (bind _max_button_location (`self.Max Button Location`))
  (bind _returnvalue (- (`self.GetButtonLocation`) (* (`self.GetButtonUpVector`) Distance)))
  (if (not (`self.Pressed`))
    (set `self.Pressed` true)
    (`self.Button Press`))
  (if (> (`KismetMathLibrary.VSize` _max_button_location) (`KismetMathLibrary.VSize` _returnvalue))
    (set `local.NewLoc` _max_button_location)
    (if (not (`self.FullyPressed`))
      (set `self.FullyPressed` true)
      (`self.Button Fully Pressed`))
    (else
      (set `local.NewLoc` _returnvalue)
      (set `self.FullyPressed` false)))
  (`SceneComponent.K2_SetWorldLocation` (`self.Cube2`) (`local.NewLoc`) false false))

(fn `ReleaseButton`
  (`SceneComponent.K2_SetWorldLocation` (`self.Cube2`) (`KismetMathLibrary.VInterpTo` (`self.GetButtonLocation`) (`self.Default Button location`) (`GameplayStatics.GetWorldDeltaSeconds`) 5.0) false false)
  (bind _output_get (set `self.Pressed` (not (`self.IsButtonAtBegin` 0.49))))
  (if (not _output_get)
    (`self.Button Release`)))

(fn `ReturnInteractableType`
  (returns (`Interact Type` :type "/Game/Blueprints/Objects/InteractType Enum"))
  (return (`self.InteractType`)))

(fn `UserConstructionScript`)