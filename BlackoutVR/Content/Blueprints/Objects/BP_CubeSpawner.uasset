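; Spawner actor that repeatedly creates Cube actors at its own location after random delays between a minimum and maximum time.
; BeginPlay starts a one-shot timer by function name on Create, which calls SpawnBlock and then ResetTimer to schedule the next randomized call.
; Spawns use a configurable scale and are skipped when the spot would collide.
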(event `self.ReceiveBeginPlay`
  (bind _returnvalue (`KismetSystemLibrary.K2_SetTimer` null "Create" (`KismetMathLibrary.RandomFloatInRange` (`self.MinSpawnTime`) (`self.MaxSpawnTime`))))
  (set `self.Timer` _returnvalue))

(fn `Create`
  (`self.SpawnBlock`)
  (`self.ResetTimer`))

(fn `ResetTimer`
  (`KismetSystemLibrary.K2_ClearAndInvalidateTimerHandle` (`self.Timer`))
  (`KismetSystemLibrary.K2_SetTimer` null "Create" (`KismetMathLibrary.RandomFloatInRange` (`self.MinSpawnTime`) (`self.MaxSpawnTime`))))

(fn `SpawnBlock`
  (`|SpawnActorFromClass` (`self.Cube`) (`KismetMathLibrary.MakeTransform` (`self.K2_GetActorLocation`) (struct) (`self.Transform scale`)) "DontSpawnIfColliding" "OverrideRootScale" null null))

(fn `UserConstructionScript`)