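; BP_ConveyorBelt is a conveyor belt actor that pushes any actor overlapping it along a horizontal direction.
; Overlap events maintain a TouchedActors list, and Tick moves each entry by a Strength-scaled push vector using a swept SetActorLocation, without delta-time scaling.
; The direction derives from the belt's yaw via sine and cosine, offset 90 degrees unless its world X exceeded Y at BeginPlay.
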(event `self.ReceiveBeginPlay`
  (bind _returnvalue (`self.GetTransform`))
  (set `self.PushX` (> (.x (.location _returnvalue)) (.y (.location _returnvalue)))))

(event `self.ReceiveActorBeginOverlap`
  (params (OtherActor :type "Actor Object Reference"))
  (`KismetArrayLibrary.Array_Add` (`self.TouchedActors`) OtherActor))

(event `self.ReceiveActorEndOverlap`
  (params (OtherActor :type "Actor Object Reference"))
  (`KismetArrayLibrary.Array_RemoveItem` (`self.TouchedActors`) OtherActor))

(event `self.ReceiveTick`
  (params (DeltaSeconds :type "Float (single-precision)"))
  (for _array_element (`self.TouchedActors`)
    (`self.MoveActor` _array_element)))

(fn `GetPushVector`
  (returns (PushVector :type "Vector Structure"))
  (bind (_returnvalue_roll _returnvalue_pitch _returnvalue_yaw) (`KismetMathLibrary.BreakRotator` (`self.K2_GetActorRotation`)))
  (if (`self.PushX`)
    (bind _vector (`self.ZRotationTo2DVector` _returnvalue_yaw))
    (return (`KismetMathLibrary.Conv_Vector2DToVector` _vector))
    (else
      (bind _vector_2 (`self.ZRotationTo2DVector` (+ _returnvalue_yaw 90.0)))
      (return (`KismetMathLibrary.Conv_Vector2DToVector` _vector_2)))))

(fn `GetStrengthVector`
  (params (PushVector :type "Vector Structure"))
  (returns (Vector :type "Vector Structure"))
  (return (* PushVector (`self.Strength`))))

(fn `UserConstructionScript`)

(fn `ZRotationTo2DVector`
  (params (Angle :type "Float (double-precision)"))
  (returns (Vector :type "Vector2D Structure"))
  (return (`KismetMathLibrary.MakeVector2D` (`KismetMathLibrary.DegSin` Angle) (`KismetMathLibrary.DegCos` Angle))))