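; Interactable light switch that, on button press, turns on a randomly picked light group through the level's StartLightHandler, found at BeginPlay.
; A timer then calls TurnOffLights to switch all three groups off and start a cooldown timer that re-enables the switch.
; The random pick uses RandomInteger(2), so only the first two groups can light up and the LightGroup3 branch is never reached.
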(event `self.OnButtonPress`
  (bind _startlighthandler (`self.StartLightHandler`))
  (if (`self.CanTurnLightOn`)
    (set `self.CanTurnLightOn` false)
    (switch `int` (`KismetMathLibrary.RandomInteger` 2)
      (:`0`
        (`/Game/Blueprints/Objects/StartLightHandler.TurnGroupOn` _startlighthandler (`/Game/Blueprints/Objects/StartLightHandler.LightGroup 1` _startlighthandler)))
      (:`1`
        (`/Game/Blueprints/Objects/StartLightHandler.TurnGroupOn` _startlighthandler (`/Game/Blueprints/Objects/StartLightHandler.LightGroup 2` _startlighthandler)))
      (:`2`
        (`/Game/Blueprints/Objects/StartLightHandler.TurnGroupOn` _startlighthandler (`/Game/Blueprints/Objects/StartLightHandler.LightGroup 3` _startlighthandler))))
    (`KismetSystemLibrary.K2_SetTimer` null "TurnOffLights" (`self.LightsTime`))))

(event `self.ReceiveBeginPlay`
  (bind _outactors (`GameplayStatics.GetAllActorsOfClass` "/Game/Blueprints/Objects/StartLightHandler.StartLightHandler_C"))
  (set `self.StartLightHandler` (`|GetArrayItem` _outactors)))

(fn `CoolDownOver`
  (set `self.CanTurnLightOn` true))

(fn `ReturnInteractableType`
  (returns (`Interact Type` :type Byte))
  (return (`self.InteractType`)))

(fn `TurnOffLights`
  (bind _startlighthandler (`self.StartLightHandler`))
  (`/Game/Blueprints/Objects/StartLightHandler.TurnGroupOff` _startlighthandler (`/Game/Blueprints/Objects/StartLightHandler.LightGroup 1` _startlighthandler))
  (`/Game/Blueprints/Objects/StartLightHandler.TurnGroupOff` _startlighthandler (`/Game/Blueprints/Objects/StartLightHandler.LightGroup 2` _startlighthandler))
  (`/Game/Blueprints/Objects/StartLightHandler.TurnGroupOff` _startlighthandler (`/Game/Blueprints/Objects/StartLightHandler.LightGroup 3` _startlighthandler))
  (`KismetSystemLibrary.K2_SetTimer` null "CoolDownOver" (`self.CooldownTime`)))

(fn `UserConstructionScript`)