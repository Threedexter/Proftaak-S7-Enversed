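; BP_ReadyButton is a pressable button that lets the VR player toggle their ready state before the game starts.
; Each press before game start flips IsReady, swaps Cube2 between red and green materials with matching custom depth stencil values, and reports the state to the GameState.
; On the GameState's InitGame event, it turns off the cube's custom depth rendering.
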(event `self.ReceiveBeginPlay`
  (`parent.ReceiveBeginPlay`)
  (bind _asexample_game_state (cast `/EnversedTouch/Example/Game/State/ExampleGameState` (`GameplayStatics.GetGameState`)))
  (add `/EnversedTouch/Example/Game/State/ExampleGameState.InitGame` _asexample_game_state (delegate `OnGameStart`)))

(event `OnGameStart`
  (`PrimitiveComponent.SetRenderCustomDepth` (`self.Cube2`) false))

(event `self.Button Press`
  (bind _cube2 (`self.Cube2`))
  (bind _cube2_2 (`self.Cube2`))
  (bind _started (message `/EnversedTouch/Example/Game/Interfaces/ExampleGMI.HasGameStarted` (`GameplayStatics.GetGameMode`)))
  (if (not _started)
    (if (`self.Is Ready`)
      (set `self.Is Ready` false)
      (`PrimitiveComponent.SetMaterial` _cube2 0 "/Game/Art/Materials/Red.Red")
      (`PrimitiveComponent.SetCustomDepthStencilValue` _cube2_2 255)
      (else
        (set `self.Is Ready` true)
        (`PrimitiveComponent.SetMaterial` _cube2 0 "/Game/Art/Materials/Green.Green")
        (`PrimitiveComponent.SetCustomDepthStencilValue` _cube2_2 60)))
    (message `/EnversedTouch/Example/Game/Interfaces/ExampleGSInterface.ReadyVRPlayer` (`GameplayStatics.GetGameState`) (`GameplayStatics.GetPlayerController` 0) (`self.Is Ready`))))

(fn `UserConstructionScript`
  (`parent.UserConstructionScript`))