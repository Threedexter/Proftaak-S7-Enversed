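; Capturable server objective that players drain of data by standing on linked trigger buttons during its game phase.
; Trigger counts toggle active state, moving the rack and switching light, sound, outline and bound cable materials.
; Looping timers drain data or slowly restore it, updating the indicator and awarding phase-scaled score, reduced for re-stolen data.
; Emptying it grants a capture bonus, disables the server and notifies GameState, possibly advancing the phase.
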(event `PlayerEnterTrigger`
  (`/Engine/EditorBlueprintResources/StandardMacros.IncrementInt` (`self.AmtOfTriggers`)
    (:`  `
      (`self.UpdateActiveState`))))

(event `PlayerExitTrigger`
  (`/Engine/EditorBlueprintResources/StandardMacros.DecrementInt` (`self.AmtOfTriggers`)
    (:`  `
      (`self.UpdateActiveState`))))

(event `PhaseChange`
  (`self.ValidatePhase` (`GameplayStatics.GetGameState`)))

(event `self.ReceiveBeginPlay`
  (bind _returnvalue (`GameplayStatics.GetGameState`))
  (bind _buttons (`self.Buttons`))
  (bind _asexample_game_state (cast `/EnversedTouch/Example/Game/State/ExampleGameState` _returnvalue))
  (add `/EnversedTouch/Example/Game/State/ExampleGameState.PhaseAdvanced` _asexample_game_state (delegate `PhaseChange`))
  (`self.ValidatePhase` _returnvalue)
  (bind _output_get (set `self.NormalPosition` (`SceneComponent.RelativeLocation` (`self.ServerRack`))))
  (`SceneComponent.K2_SetRelativeLocation` (`self.ServerRack`) _output_get false false)
  (if (> (`KismetArrayLibrary.Array_Length` _buttons) 0)
    (for _array_element _buttons
      (add `/Game/Blueprints/Objects/BP_PressurePad.OnPlayerEnterTrigger` _array_element (delegate `PlayerEnterTrigger`))
      (add `/Game/Blueprints/Objects/BP_PressurePad.OnPlayerExitTrigger` _array_element (delegate `PlayerExitTrigger`))
      (set `self.RisenPosition` (`self.AddOffsetToVectorDown` (`self.RiseCoëf`)))
      (set `self.HiddenPosition` (`self.AddOffsetToVectorUp` 200.0))
      (bind _asserver_indictator (cast `/Game/Art/UI/ServerIndictator` (`WidgetComponent.GetUserWidgetObject` (`self.Widget`))))
      (set `self.ServerIndicator` _asserver_indictator)
      (set `self.DataInStorage` (`self.DataMax`)))))

(event `self.ReceiveTick`
  (params (DeltaSeconds :type "Float (single-precision)"))
  (bind _capturebeat (`self.CaptureBeat`))
  (`|ExecutionSequence`
    (:`then_0`
      (if (`self.IsCaptured`)
        (`SceneComponent.K2_SetRelativeLocation` (`self.ServerRack`) (`self.VectorInterp` (`SceneComponent.RelativeLocation` (`self.ServerRack`)) (`self.HiddenPosition`)) false false)
        (else
          ;[1 1 1] Handle Server Actions
          (if (`self.IsActive`)
            (`SceneComponent.K2_SetRelativeLocation` (`self.ServerRack`) (`self.VectorInterp` (`SceneComponent.RelativeLocation` (`self.ServerRack`)) (`self.RisenPosition`)) false false)
            (`/Engine/EditorBlueprintResources/StandardMacros.DoOnce` false :!label _label
              (:`Completed`
                (bind _returnvalue (`KismetSystemLibrary.K2_SetTimerDelegate` (delegate `CaptureLoop`) 0.5 true))
                (set `self.CaptureBeat` _returnvalue)
                (`self.SetActiveLight`)
                (`KismetSystemLibrary.K2_ClearAndInvalidateTimerHandle` (stale _returnvalue_2))
                (`self.PlaySound` true)
                (`self.SetBindedCables` "NewEnumerator2")))
            (else
              (`SceneComponent.K2_SetRelativeLocation` (`self.ServerRack`) (`self.VectorInterp` (`SceneComponent.RelativeLocation` (`self.ServerRack`)) (`self.NormalPosition`)) false false)
              (`|ExecutionSequence`
                (:`then_0`
                  (goto _label :!via `Reset`))
                (:`then_1`
                  (`self.SetInactiveLight`)
                  (if (`KismetSystemLibrary.K2_IsValidTimerHandle` _capturebeat)
                    (`KismetSystemLibrary.K2_ClearAndInvalidateTimerHandle` _capturebeat)))
                (:`then_2`
                  (`/Engine/EditorBlueprintResources/StandardMacros.DoOnce` false :!label _label_2
                    (:`Completed`
                      (bind _returnvalue_2 (`KismetSystemLibrary.K2_SetTimerDelegate` (delegate `Resetloop`) 1.0 true))
                      (`self.PlaySound` false)
                      (`self.SetBindedCables` "NewEnumerator1"))))))))))))

(event `CaptureLoop`
  ;[1 1 1] Handle Server Actions
  (`self.RemoveData`)
  (goto _label_2 :!via `Reset`))

(event `Resetloop`
  (`self.MutateData` (`KismetMathLibrary.FTrunc` (* (`self.TransferRate`) -0.2))))

(event `/Game/Blueprints/Objects/ServerBindInterface.Bind`
  (params (Cable :type "/Game/Blueprints/Objects/BP_Cable Object Reference"))
  (`KismetArrayLibrary.Array_AddUnique` (`self.Cables`) Cable))

(event `/Game/Blueprints/Objects/ServerBindInterface.Unbind`
  (params (Cable :type "/Game/Blueprints/Objects/BP_Cable Object Reference"))
  (`KismetArrayLibrary.Array_RemoveItem` (`self.Cables`) Cable))

(fn `DisableServer`
  (bind _returnvalue (`GameplayStatics.GetGameState`))
  (set `self.IsActive` false)
  (`KismetSystemLibrary.K2_ClearAndInvalidateTimerHandle` (`self.CaptureBeat`))
  (set `self.IsCaptured` true)
  (`self.SetOutline` 0)
  (`self.SetBindedCables` "NewEnumerator0")
  (message `/EnversedTouch/Example/Game/Interfaces/ExampleGSInterface.TriggerPhaseCount` _returnvalue)
  (bind _trigger (message `/EnversedTouch/Example/Game/Interfaces/ExampleGSInterface.ShouldAdvancePhase` _returnvalue))
  (if _trigger
    (message `/EnversedTouch/Example/Game/Interfaces/ExampleGSInterface.AdvancePhase` _returnvalue)))

(fn `GiveScore`
  (params (score :type Integer))
  (for _array_element (`self.Buttons`)
    (bind _players (`/Game/Blueprints/Objects/BP_PressurePad.GetPlayers` _array_element))
    (for _array_element_2 _players
      (`ExampleScore.AddToScore` _array_element_2 score))))

(fn `MutateData`
  (params (`Negative mutation` :type Integer :default 0))
  (bind _returnvalue (`KismetMathLibrary.Conv_IntToDouble` (`self.DataMax`)))
  (bind _output_get (set `self.DataInStorage` (`KismetMathLibrary.FTrunc` (`KismetMathLibrary.MapRangeClamped` (`KismetMathLibrary.Conv_IntToDouble` (- (`self.DataInStorage`) `Negative mutation`)) 0.0 _returnvalue 0.0 _returnvalue))))
  (`/Game/Art/UI/ServerIndictator.UpdateBar` (`self.ServerIndicator`) (`KismetMathLibrary.MapRangeClamped` (`KismetMathLibrary.Conv_IntToDouble` (- (`self.DataMax`) (`self.DataInStorage`))) 0.0 100.0 0.0 1.0))
  (bind _score_multiplier (`self.UpdateStolenDataIfNecessary`))
  (bind _phase (message `/EnversedTouch/Example/Game/Interfaces/ExampleGSInterface.GetPhase` (`GameplayStatics.GetGameState`)))
  (bind (_sps _cs) (`self.AdjustScoresToMultiplier` (* _score_multiplier (- (+ (/ (`KismetMathLibrary.Conv_IntToDouble` _phase) 5.0) 1.0) 0.2))))
  (`self.GiveScore` _sps)
  (if (<= _output_get 0)
    (`self.GiveScore` _cs)
    (`self.DisableServer`)))

(fn `PlaySound`
  (params (Rising :type Boolean))
  (bind _speaker (`self.Speaker`))
  (bind _returnvalue (`AudioComponent.IsPlaying` _speaker))
  (if Rising
    (if _returnvalue
      (`AudioComponent.Stop` _speaker))
    (`AudioComponent.SetSound` _speaker "/Game/Sound/ServerRiserFinal_Cue.ServerRiserFinal_Cue")
    (`AudioComponent.Play` _speaker 0.0)
    (else
      (if _returnvalue
        (`AudioComponent.Stop` _speaker))
      (`AudioComponent.SetSound` _speaker "/Game/Sound/ServerFallFinal_Cue.ServerFallFinal_Cue")
      (`AudioComponent.Play` _speaker 0.0))))

(fn `RemoveData`
  (`self.MutateData` (`self.TransferRate`)))

(fn `SetActiveLight`
  (`LightComponent.SetLightColor` (`self.PointLight`) (struct :`R` 1.0 :`A` 1.0) true))

(fn `SetBindedCables`
  (params (Cable :type "/Game/Blueprints/Objects/EServerCable Enum" :default "NewEnumerator2"))
  (for _array_element (`self.Cables`)
    (message `/Game/Blueprints/Objects/ServerCableInterface.SetMaterial` _array_element Cable)))

(fn `SetInactiveLight`
  (`LightComponent.SetLightColor` (`self.PointLight`) (struct :`G` 1.0 :`B` 1.0 :`A` 1.0) true))

(fn `SetOutline`
  (params (`Outline Colour` :type Integer))
  (bind _cube (`self.Cube`))
  (if (== `Outline Colour` 0)
    (`PrimitiveComponent.SetRenderCustomDepth` _cube false)
    (`PrimitiveComponent.SetRenderCustomDepth` (`self.ServerRack`) false)
    (else
      (`PrimitiveComponent.SetRenderCustomDepth` (`self.ServerRack`) true)
      (`PrimitiveComponent.SetRenderCustomDepth` _cube true)
      (`PrimitiveComponent.SetCustomDepthStencilValue` _cube `Outline Colour`)
      (`PrimitiveComponent.SetCustomDepthStencilValue` (`self.ServerRack`) `Outline Colour`))))

(fn `UpdateStolenDataIfNecessary`
  (returns (`Score Multiplier` :type "Float (double-precision)"))
  (bind _returnvalue (- (`self.DataMax`) (`self.DataInStorage`)))
  (if (< (`self.StoleHigh`) _returnvalue)
    (set `self.StoleHigh` _returnvalue)
    (return 1.0)
    (else
      (return (`self.DataNerf`)))))

(fn `UserConstructionScript`
  (locals (NumberOfSplinePoints :type Integer)))

(fn `ValidatePhase`
  (params (`Game State` :type "Object Object Reference"))
  (bind _phase (message `/EnversedTouch/Example/Game/Interfaces/ExampleGSInterface.GetPhase` `Game State`))
  (bind _output_get (set `self.IsCaptured` (not (and (== _phase (`self.Phase`)) (== (`self.StoleHigh`) -1)))))
  (if _output_get
    (`self.SetOutline` 0)
    (`self.SetBindedCables` "NewEnumerator0")
    (else
      (`self.SetOutline` 128)
      (`self.SetBindedCables` "NewEnumerator1"))))