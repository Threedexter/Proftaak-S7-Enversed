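; Spectator capture actor that shows a render target on the VR spectator screen and feeds touch-actor screen positions to its SpectatorUI widget.
; On BeginPlay, if enabled, it fetches touch actors from the GameMode and traces two opposite screen corners to calibrate world-space edges.
; Each Tick it traces from the capture component to each actor, remaps hit X/Y to clamped, axis-swapped 1920x1080 coordinates, and passes them with player IDs to the widget.
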(event `self.ReceiveBeginPlay`
  (bind _asspectator_ui (cast `/Game/Art/UI/SpectatorUI` (`WidgetComponent.GetUserWidgetObject` (`self.Widget`))))
  (set `self.PlayerUI` _asspectator_ui)
  (set `self.RaySpread` 1.78)
  (set `self.RayOffset` 0.0)
  (if (`self.EnableSpectatorScreen`)
    (`HeadMountedDisplayFunctionLibrary.SetSpectatorScreenMode` "Texture")
    (`HeadMountedDisplayFunctionLibrary.SetSpectatorScreenTexture` "/Game/Art/Spectator/SpecScreenRendTarget.SpecScreenRendTarget")
    (bind _touch_actors (message `/Game/Blueprints/GameMode/Interfaces/IBlackoutGM.GetAllTouchActors` (`GameplayStatics.GetGameMode`)))
    (set `self.TouchActors` _touch_actors)
    (`|ExecutionSequence`
      (:`then_0`
        (`self.RayCastWorldCoords` (0.0 0.0)))
      (:`then_1`
        (`self.RayCastWorldCoords` (1920.0 1080.0))))
    (else
      (`HeadMountedDisplayFunctionLibrary.SetSpectatorScreenMode` "SingleEye"))))

(event `self.ReceiveTick`
  (params (DeltaSeconds :type "Float (single-precision)"))
  (for (_array_element _array_index) (`self.TouchActors`)
    (bind (_outhit _returnvalue) (`KismetSystemLibrary.LineTraceSingle` :`Start` (`SceneComponent.K2_GetComponentLocation` (`self.CaptureComponent2D`)) :`End` (`SceneComponent.K2_GetComponentLocation` (`MovementActor.collisionBox` _array_element)) :`TraceChannel` "TraceTypeQuery3" :`bIgnoreSelf` false))
    (if _returnvalue
      (bind (_bblockinghit _binitialoverlap _time _location) (`GameplayStatics.BreakHitResult` _outhit))
      (bind _screen_location (`self.GetScreenLocationFromWorldSpaceClamped` (`KismetMathLibrary.MakeVector2D` (.x _location) (.y _location))))
      (`KismetArrayLibrary.Array_AddUnique` (`self.Players`) (make `/Game/Blueprints/PlayerUIStruct` _screen_location _array_index))))
  (set `/Game/Art/UI/SpectatorUI.TouchActors` (`self.Players`) (`self.PlayerUI`))
  (`KismetArrayLibrary.Array_Clear` (`self.Players`)))

(fn `GetScreenLocationFromWorldSpaceClamped`
  (params (WorldLocation :type "Vector2D Structure"))
  (returns (`Screen Location` :type "Vector2D Structure"))
  (bind (_output_x _output_y) (`KismetMathLibrary.BreakVector2D` (`|GetArrayItem` (`self.ScreenEdges`))))
  (bind (_output_x_2 _output_y_2) (`KismetMathLibrary.BreakVector2D` (`|GetArrayItem` (`self.ScreenEdges`) 1)))
  (bind _output_x_3 (`KismetMathLibrary.BreakVector2D` (`|GetArrayItem` (`self.ScreenEdges`) 1)))
  (bind _output_x_4 (`KismetMathLibrary.BreakVector2D` (`|GetArrayItem` (`self.ScreenEdges`))))
  (return (`KismetMathLibrary.MakeVector2D` (`KismetMathLibrary.MapRangeClamped` WorldLocation_Y _output_y _output_y_2 0.0 1920.0) (`KismetMathLibrary.MapRangeClamped` WorldLocation_X _output_x_4 _output_x_3 0.0 1080.0))))

(fn `RayCastWorldCoords`
  (params (ScreenCoords :type "Vector2D Structure"))
  (bind _returnvalue (`self.K2_GetActorLocation`))
  (bind _worldlocation (`self.ScreenToSieWorld` (`KismetMathLibrary.MakeVector2D` ScreenCoords_X ScreenCoords_Y)))
  (bind (_returnvalue_x _returnvalue_y _returnvalue_z) (`KismetMathLibrary.BreakVector` (`KismetMathLibrary.GreaterGreater_VectorRotator` _worldlocation (struct :`Yaw` 270.0))))
  (bind _outhit (`KismetSystemLibrary.LineTraceSingle` :`Start` _returnvalue :`End` (- _returnvalue (* (`KismetMathLibrary.MakeVector` (+ (/ (* _returnvalue_x -1.0) (`self.raySpread`)) (`self.rayOffset`)) _returnvalue_y _returnvalue_z) 10000.0)) :`TraceChannel` "TraceTypeQuery3" :`bIgnoreSelf` false :`TraceColor` (struct :`R` 1.0 :`B` 0.014997 :`A` 1.0) :`DrawTime` 3000.0))
  (bind (_bblockinghit _binitialoverlap _time _location) (`GameplayStatics.BreakHitResult` _outhit))
  (`KismetArrayLibrary.Array_AddUnique` (`self.ScreenEdges`) (`KismetMathLibrary.MakeVector2D` (.x _location) (.y _location))))

(fn `UserConstructionScript`)