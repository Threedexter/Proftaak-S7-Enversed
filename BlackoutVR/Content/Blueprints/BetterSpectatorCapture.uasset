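; Spectator capture actor for the Blackout VR game that puts a render target on the spectator screen, when enabled, and manages its touch-driven UI.
; Game mode start and end events switch its widgets to spectator or score screen, while player pawn touches become pointer clicks.
; Each tick, it line-traces toward touch actors and feeds hits into WidgetInteraction, passing 2D widget positions, scores and IDs to SpectatorUI.
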(event `self.ReceiveTick`
  (params (DeltaSeconds :type "Float (single-precision)"))
  (`self.DrawUITouchActors`))

(event `TouchedLocation`
  (params (TouchLocation :type "Vector2D Structure") (IsTouch :type Boolean))
  (bind _widgetinteraction (`self.widgetInteraction`))
  (bind _touchkeypress (`self.TouchKeyPress`))
  ;[1 1 1] Working touchedlocation
  (if IsTouch
    (bind (_touchlocationwidget _touchlocationworld _returnvalue) (`self.CheckIfTouchedWidgetFromCamera` TouchLocation (`self.TouchDistance`)))
    (if _returnvalue
      (`WidgetInteractionComponent.PressPointerKey` _widgetinteraction _touchkeypress)
      (`WidgetInteractionComponent.ReleasePointerKey` _widgetinteraction _touchkeypress))))

(event `StartGameSpec`
  (bind _widgetmenu (`self.WidgetMenu`))
  (bind _widgetspec (`self.WidgetSpec`))
  ;[1 1 1] OnStartGame Happens when you start a game
  (`SceneComponent.SetVisibility` _widgetmenu false false)
  (`PrimitiveComponent.SetCollisionEnabled` _widgetmenu "NoCollision")
  (`SceneComponent.SetVisibility` _widgetspec true false)
  (`PrimitiveComponent.SetCollisionEnabled` _widgetspec "QueryOnly"))

(event `EndGameEvent`
  (bind _widgetspec (`self.WidgetSpec`))
  (bind _widgetend (`self.WidgetEnd`))
  (bind _widgetmenu (`self.WidgetMenu`))
  ;[1 1 1] Happens when a game ends
  (`SceneComponent.SetVisibility` _widgetspec false false)
  (`PrimitiveComponent.SetCollisionEnabled` _widgetspec "NoCollision")
  (`SceneComponent.SetVisibility` _widgetmenu false false)
  (`PrimitiveComponent.SetCollisionEnabled` _widgetmenu "NoCollision")
  (`SceneComponent.SetVisibility` _widgetend true false)
  (`PrimitiveComponent.SetCollisionEnabled` _widgetend "QueryOnly")
  (bind _asscore_screen (cast `/Game/Art/UI/ScoreScreen` (`WidgetComponent.GetUserWidgetObject` _widgetend)))
  (`/Game/Art/UI/ScoreScreen.SetAllAscores` _asscore_screen))

(event `self.ReceiveBeginPlay`
  ;[1 1 1] Beginplay
  (bind _asblackout_gm (cast `/Game/Blueprints/GameMode/Blackout_GM` (`GameplayStatics.GetGameMode`))
    (:`then`
      (add `/Game/Blueprints/GameMode/Blackout_GM.GameStartED` _asblackout_gm (delegate `StartGameSpec`))
      (add `/Game/Blueprints/GameMode/Blackout_GM.GameEndED` _asblackout_gm (delegate `EndGameEvent`)))
    (:`CastFailed`
      _))
  (bind _asblackout_vrcharacter (cast `BlackoutVRCharacter` (`GameplayStatics.GetPlayerPawn` 0))
    (:`then`
      (bind _output_get (set `self.PlayerPawn` _asblackout_vrcharacter))
      (add `BlackoutVRCharacter.onTouchUpdate` _output_get (delegate `TouchedLocation`)))
    (:`CastFailed`
      _))
  (bind _asspectator_ui (cast `/Game/Art/UI/SpectatorUI` (`WidgetComponent.GetUserWidgetObject` (`self.WidgetSpec`))))
  (set `self.PlayerUI` _asspectator_ui)
  (if (`self.EnableSpectatorScreen`)
    (`HeadMountedDisplayFunctionLibrary.SetSpectatorScreenMode` "Texture")
    (`HeadMountedDisplayFunctionLibrary.SetSpectatorScreenTexture` "/Game/Art/Spectator/SpecScreenRendTarget.SpecScreenRendTarget")
    (else
      (`HeadMountedDisplayFunctionLibrary.SetSpectatorScreenMode` "Disabled")))
  (`/Engine/EditorBlueprintResources/StandardMacros.IsValid` (`self.widgetInteraction`)
    (:`Is Valid`
      (`KismetSystemLibrary.PrintString` (`KismetStringLibrary.Conv_VectorToString` (`self.K2_GetActorLocation`))))
    (:`Is Not Valid`
      (`KismetSystemLibrary.PrintString` "Ik ben Unreal en ik ben eigenwijs"))))

(event `DrawUITouchActors`
  (bind _widgetinteraction (`self.widgetInteraction`))
  ;[1 1 1] Updates the UI touch actors
  (bind _touch_actors (message `/Game/Blueprints/GameMode/Interfaces/IBlackoutGM.GetAllTouchActors` (`GameplayStatics.GetGameMode`)))
  (if (> (`KismetArrayLibrary.Array_Length` _touch_actors) 0)
    (for _array_element _touch_actors
      (bind _returnvalue (`TouchActor.GetTouchActorID` _array_element))
      (bind _outhit (`KismetSystemLibrary.LineTraceSingle` :`Start` (`self.K2_GetActorLocation`) :`End` (`self.K2_GetActorLocation` _array_element) :`TraceChannel` "TraceTypeQuery3" :`bIgnoreSelf` false :`TraceColor` (struct :`G` 1.0 :`B` 0.024281 :`A` 1.0)))
      (`SpectatorWidgetInteraction.SetCustomHitResultAndUpdate` _widgetinteraction _outhit)
      (if (or (`WidgetInteractionComponent.IsOverInteractableWidget` _widgetinteraction) (`WidgetInteractionComponent.IsOverFocusableWidget` _widgetinteraction))
        (`KismetArrayLibrary.Array_AddUnique` (`self.Players`) (make `/Game/Blueprints/PlayerUIStruct` (`WidgetInteractionComponent.Get2DHitLocation` _widgetinteraction) (`TouchPawn.currentScore` _array_element) _returnvalue))))
    (set `/Game/Art/UI/SpectatorUI.TouchActors` (`self.Players`) (`self.PlayerUI`))
    (`KismetArrayLibrary.Array_Clear` (`self.Players`))))

(fn `UserConstructionScript`)