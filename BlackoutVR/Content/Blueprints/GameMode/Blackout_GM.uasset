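; Game mode for Blackout that spawns the VR player and touch actors and runs game start and stop.
; Player zero gets a VR pawn, or a non-VR one under DebugPawn, at an available VR spawn point.
; StartGame spawns one touch pawn per area index, fades start lights and notifies game state and player.
; Spawn points are cached by class and picked randomly among available ones; respawns teleport touch actors within their ID's area.
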(event `self.SpawnTouchActors`
  (params (Amount :type Integer))
  ;[1 1 1] Spawns touch actors when there are spawn points
  (for _index (range Amount)
    (bind _spawnpoint (`self.GetAvailableSpawnPointsOfArea` _index))
    (`/Engine/EditorBlueprintResources/StandardMacros.IsValid` _spawnpoint
      (:`Is Valid`
        (message `/Game/Blueprints/Spawn/Interfaces/SpawnInterface.SetSpawned` _spawnpoint)
        (bind _spawnpoint_2 (`/Game/Blueprints/Spawn/SpawnPoint.GetSpawnPoint` _spawnpoint))
        (bind _returnvalue (`|SpawnActorFromClass` "/Game/Blueprints/TouchActor/MyTouchPawn.MyTouchPawn_C" (`KismetMathLibrary.MakeTransform` (.location _spawnpoint_2) (.rotation _spawnpoint_2)) "AdjustIfPossibleButAlwaysSpawn" "OverrideRootScale" null null))
        (bind _output_get (set `/Game/Blueprints/TouchActor/MyTouchPawn.TouchActorID` _index _returnvalue))
        (`ScoreKeeper.SetCName` _returnvalue _output_get)
        (`KismetArrayLibrary.Array_AddUnique` (`self.TouchActors`) _returnvalue)))))

(event `self.RespawnTouchActor`
  (params (TouchActor :type "Actor Object Reference"))
  ;[1 1 1] Respawns touch actor
  (bind _asbp_touch_actor (cast `/Game/Blueprints/TouchActor/BP_TouchActor` TouchActor))
  (bind _spawnpoint (`self.GetAvailableSpawnPointsOfArea` (`/Game/Blueprints/TouchActor/BP_TouchActor.TouchActorID` _asbp_touch_actor)))
  (`/Engine/EditorBlueprintResources/StandardMacros.IsValid` _spawnpoint
    (:`Is Valid`
      (`/Game/Blueprints/Spawn/Interfaces/SpawnInterface.SetSpawned` _spawnpoint)
      (bind _spawnpoint_2 (`/Game/Blueprints/Spawn/SpawnPoint.GetSpawnPoint` _spawnpoint))
      (`self.K2_SetActorTransform` TouchActor (`KismetMathLibrary.MakeTransform` (.location _spawnpoint_2) (.rotation _spawnpoint_2)) false true))
    (:`Is Not Valid`
      (`KismetSystemLibrary.PrintString` "No Vali SpawnPoint"))))

(event `self.SpawnVRPlayer`
  (params (Controller :type "Controller Object Reference"))
  ;[1 1 1] Spawns the VR Player
  (if (`self.DebugPawn`)
    (bind _vrspawnpoint (`self.GetAvailableVRSpawnPoint`))
    (`/Engine/EditorBlueprintResources/StandardMacros.IsValid` _vrspawnpoint
      (:`Is Valid`
        (`/Game/Blueprints/Spawn/VRSpawnPoint.SetSpawned` _vrspawnpoint)
        (bind _spawnpoint (`/Game/Blueprints/Spawn/Interfaces/SpawnInterface.GetSpawnPoint` _vrspawnpoint))
        (bind _returnvalue (`|SpawnActorFromClass` "/Game/Blueprints/Pawn/BlackoutNonVRInheritedPAwn.BlackoutNonVRInheritedPawn_C" (`KismetMathLibrary.MakeTransform` (.location _spawnpoint) (.rotation _spawnpoint)) "AdjustIfPossibleButAlwaysSpawn" "OverrideRootScale" null null))
        (`Controller.Possess` Controller _returnvalue)))
    (else
      (bind _vrspawnpoint_2 (`self.GetAvailableVRSpawnPoint`))
      (`/Engine/EditorBlueprintResources/StandardMacros.IsValid` _vrspawnpoint_2
        (:`Is Valid`
          (`/Game/Blueprints/Spawn/VRSpawnPoint.SetSpawned` _vrspawnpoint_2)
          (bind _spawnpoint_2 (`/Game/Blueprints/Spawn/Interfaces/SpawnInterface.GetSpawnPoint` _vrspawnpoint_2))
          (bind _returnvalue_2 (`|SpawnActorFromClass` "/Game/Blueprints/Pawn/BlackoutVRPawn.BlackoutVRPawn_C" (`KismetMathLibrary.MakeTransform` (.location _spawnpoint_2) (.rotation _spawnpoint_2)) "AdjustIfPossibleButAlwaysSpawn" "OverrideRootScale" null null))
          (`Controller.Possess` Controller _returnvalue_2))))))

(event `self.StartGame`
  ;[1 1 1] Start game
  (if (not (`self.startedGame`))
    (set `self.startedGame` true)
    (`self.SpawnTouchActors` (`self.AmountOfTouchActors`))
    (message `/Game/Blueprints/GameState/Interfaces/IBlackoutGameState.StartGame` (`GameplayStatics.GetGameState`))
    (bind _outactors (`GameplayStatics.GetAllActorsOfClass` "/Game/Blueprints/StartLightHandler.StartLightHandler_C"))
    (if (> (`KismetArrayLibrary.Array_Length` _outactors) 0)
      (`/Game/Blueprints/StartLightHandler.StartFade` (`|GetArrayItem` _outactors)))
    (`self.GameStartED`)
    (`KismetSystemLibrary.Delay` 0.2)
    (message `/Game/Blueprints/Pawn/LekkebezigUnreal.StartGame` (`Controller.K2_GetPawn` (`GameplayStatics.GetPlayerController` 0)))))

(event `self.StopGame`
  ;[1 1 1] Stop game
  (message `/Game/Blueprints/Pawn/LekkebezigUnreal.StopGame` (`GameplayStatics.GetPlayerPawn` 0))
  (`self.GameEndED`)
  (set `self.startedGame` false))

(fn `FindPlayerStart`
  (params (Player :type "Controller Object Reference") (IncomingName :type String))
  (returns (ReturnValue :type "Actor Object Reference"))
  (bind _vrspawnpoint (`self.GetAvailableVRSpawnPoint`))
  (`/Engine/EditorBlueprintResources/StandardMacros.IsValid` _vrspawnpoint
    (:`Is Valid`
      (return _vrspawnpoint))
    (:`Is Not Valid`
      (return null))))

(fn `GetAllTouchActors`
  (returns (`Touch Actors` :type "Array of /Game/Blueprints/TouchActor/MyTouchPawn Object Reference"))
  (return (`self.TouchActors`)))

(fn `GetAvailableSpawnPoint`
  (returns (SpawnPoint :type "/Game/Blueprints/Spawn/SpawnPoint Object Reference"))
  (locals (NewSpawnPoints :type "Array of /Game/Blueprints/Spawn/SpawnPoint Object Reference"))
  (bind _newspawnpoints (`local.NewSpawnPoints`))
  (bind _spawnpoints (`self.SpawnPoints`))
  (bind _returnvalue (`KismetArrayLibrary.Array_Length` _newspawnpoints))
  (if (not (> (`KismetArrayLibrary.Array_Length` (`self.SpawnPoints`)) 0))
    (bind _outactors (`GameplayStatics.GetAllActorsOfClass` "/Game/Blueprints/Spawn/SpawnPoint.SpawnPoint_C"))
    (set `self.SpawnPoints` _outactors))
  (for _array_element _spawnpoints
    (bind _spawnable (`/Game/Blueprints/Spawn/SpawnPoint.CanSpawn` _array_element))
    (if _spawnable
      (`KismetArrayLibrary.Array_Add` (`local.NewSpawnPoints`) _array_element)))
  (if (> _returnvalue 0)
    (return (`|GetArrayItem` _newspawnpoints (`KismetMathLibrary.RandomIntegerInRange` 0 (- _returnvalue 1))))
    (elif (> (`KismetArrayLibrary.Array_Length` _spawnpoints) 0)
      (return (`|GetArrayItem` _spawnpoints))
      (else
        (return null)))))

(fn `GetAvailableSpawnPointsOfArea`
  (params (Area :type Integer))
  (returns (SpawnPoint :type "/Game/Blueprints/Spawn/SpawnPoint Object Reference"))
  (locals (NewSpawnPoints :type "Array of /Game/Blueprints/Spawn/SpawnPoint Object Reference"))
  (bind _newspawnpoints (`local.NewSpawnPoints`))
  (bind _returnvalue (`KismetArrayLibrary.Array_Length` _newspawnpoints))
  (bind _spawnpoints (`self.GetSpawnPointsOfArea` Area))
  (for _array_element _spawnpoints
    (bind _spawnable (`/Game/Blueprints/Spawn/SpawnPoint.CanSpawn` _array_element))
    (if _spawnable
      (`KismetArrayLibrary.Array_Add` (`local.NewSpawnPoints`) _array_element)))
  (if (> _returnvalue 0)
    (return (`|GetArrayItem` _newspawnpoints (`KismetMathLibrary.RandomIntegerInRange` 0 (- _returnvalue 1))))
    (else
      (return (`|GetArrayItem` _newspawnpoints)))))

(fn `GetAvailableVRSpawnPoint`
  (returns (VRSpawnPoint :type "/Game/Blueprints/Spawn/VRSpawnPoint Object Reference"))
  (locals (NewVRSpawnPoint :type "Array of /Game/Blueprints/Spawn/VRSpawnPoint Object Reference"))
  (bind _vrspawnpoints (`self.VRSpawnPoints`))
  (bind _newvrspawnpoint (`local.NewVRSpawnPoint`))
  (bind _returnvalue (`KismetArrayLibrary.Array_Length` _newvrspawnpoint))
  (if (not (> (`KismetArrayLibrary.Array_Length` (`self.VRSpawnPoints`)) 0))
    (bind _outactors (`GameplayStatics.GetAllActorsOfClass` "/Game/Blueprints/Spawn/VRSpawnPoint.VRSpawnPoint_C"))
    (set `self.VRSpawnPoints` _outactors))
  (for _array_element (`self.VRSpawnPoints`)
    (bind _spawnable (`/Game/Blueprints/Spawn/Interfaces/SpawnInterface.CanSpawn` _array_element))
    (if _spawnable
      (`KismetArrayLibrary.Array_Add` (`local.NewVRSpawnPoint`) _array_element)))
  (if (> _returnvalue 0)
    (return (`|GetArrayItem` _newvrspawnpoint (`KismetMathLibrary.RandomIntegerInRange` 0 (- _returnvalue 1))))
    (elif (> (`KismetArrayLibrary.Array_Length` _vrspawnpoints) 0)
      (return (`|GetArrayItem` _vrspawnpoints))
      (else
        (return null)))))

(fn `GetDefaultPawnClassForController`
  (params (InController :type "Controller Object Reference"))
  (returns (ReturnValue :type "Object Class Reference"))
  (bind _asplayer_controller (cast `PlayerController` InController)
    (:`then`
      (bind _returnvalue (`GameplayStatics.GetPlayerControllerID` _asplayer_controller))
      (if (== _returnvalue 0)
        (if (`self.DebugPawn`)
          (return "/Game/Blueprints/Pawn/BlackoutNonVRInheritedPAwn.BlackoutNonVRInheritedPawn_C")
          (else
            (return "/Game/Blueprints/Pawn/BlackoutVRPawn.BlackoutVRPawn_C")))
        (else
          _)))
    (:`CastFailed`
      _))
  (return (`self.DefaultPawnClass`)))

(fn `GetSpawnPointsOfArea`
  (params (Area :type Integer))
  (returns (SpawnPoints :type "Array of /Game/Blueprints/Spawn/SpawnPoint Object Reference"))
  (locals (NewSpawnPoints :type "Array of /Game/Blueprints/Spawn/SpawnPoint Object Reference"))
  (bind _spawn_points (`self.GetSpawnPoints`))
  (for _array_element _spawn_points
    (bind _belongsto (`/Game/Blueprints/Spawn/SpawnPoint.BelongsToArea` _array_element Area))
    (if _belongsto
      (`KismetArrayLibrary.Array_Add` (`local.NewSpawnPoints`) _array_element)))
  (return (`local.NewSpawnPoints`)))

(fn `UserConstructionScript`)