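; Spawn point actor that reports whether a player can spawn there and supplies the spawn transform, flagged as non-VR.
; Availability follows SpawnBox overlaps and explicit set/reset events: any begin overlap blocks it, any end overlap frees it.
; GetSpawnPoint returns the actor's transform lowered on Z with unit scale.
; Cooldown time and timer-clearing events exist, but the timer that would reset the point is disconnected.
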(event `/Game/Blueprints/Spawn/Interfaces/SpawnInterface.SetCooldownTime`
  (params (Time :type "Float (single-precision)"))
  ;[1 1 1] Sets the cooldown time
  (set `self.CooldownTime` Time))

(event `/Game/Blueprints/Spawn/Interfaces/SpawnInterface.SetSpawned`
  ;[1 1 1] Sets the player to spawned
  (set `self.CanPlayerSpawn` false))

(event `/Game/Blueprints/Spawn/Interfaces/SpawnInterface.ResetSpawnPoint`
  ;[1 1 1] Resets the spawnpoint
  (set `self.CanPlayerSpawn` true))

(event `/Game/Blueprints/Spawn/Interfaces/SpawnInterface.ResetCooldown`
  ;[1 1 1] Reset function
  (`KismetSystemLibrary.K2_ClearAndInvalidateTimerHandle` (`self.CooldownTimer`)))

(event `self.SpawnBox.OnComponentEndOverlap`
  (params (OverlappedComponent :type "PrimitiveComponent Object Reference") (OtherActor :type "Actor Object Reference") (OtherComp :type "PrimitiveComponent Object Reference") (OtherBodyIndex :type Integer))
  ;[1 1 1] Overlap
  (set `self.CanPlayerSpawn` true))

(event `self.SpawnBox.OnComponentBeginOverlap`
  (params (OverlappedComponent :type "PrimitiveComponent Object Reference") (OtherActor :type "Actor Object Reference") (OtherComp :type "PrimitiveComponent Object Reference") (OtherBodyIndex :type Integer) (bFromSweep :type Boolean) (SweepResult :type "HitResult Structure (by ref)"))
  ;[1 1 1] Overlap
  (set `self.CanPlayerSpawn` false))

(fn `CanSpawn`
  (returns (Spawnable :type Boolean))
  (return (`self.CanPlayerSpawn`)))

(fn `GetSpawnPoint`
  (returns (SpawnPoint :type "Transform Structure"))
  (bind _returnvalue (`self.GetTransform`))
  (return (`KismetMathLibrary.MakeTransform` (`KismetMathLibrary.MakeVector` (.x (.location _returnvalue)) (.y (.location _returnvalue)) (- (.z (.location _returnvalue)) 40.0)) (.rotation _returnvalue))))

(fn `IsVRSpawn`
  (returns (VRspawn :type Boolean))
  (return false))

(fn `UserConstructionScript`)