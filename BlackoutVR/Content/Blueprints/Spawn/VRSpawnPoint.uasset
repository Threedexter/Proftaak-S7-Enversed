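; VR player spawn point that reports whether it is free and where the player should appear.
; SpawnBox overlaps and the SetSpawned and ResetSpawnPoint events toggle the availability flag returned by CanSpawn.
; GetSpawnPoint drops the actor transform to the root capsule's bottom with unit scale.
; It identifies as VR and belongs to no area; cooldown time is stored, but the timer that would use it is unconnected.
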(event `/Game/Blueprints/Spawn/Interfaces/SpawnInterface.SetCooldownTime`
  (params (Time :type "Float (single-precision)"))
  ;[1 1 1] Sets the cooldown time
  (set `self.CooldownTime` Time))

(event `/Game/Blueprints/Spawn/Interfaces/SpawnInterface.SetSpawned`
  ;[1 1 1] Sets the player to spawned
  (set `self.CanPlayerSpawn` false))

(event `/Game/Blueprints/Spawn/Interfaces/SpawnInterface.ResetSpawnPoint`
  ;[1 1 1] Resets the spawnpoint
  (set `self.CanPlayerSpawn` true))

(event `/Game/Blueprints/Spawn/Interfaces/SpawnInterface.ResetCooldown`
  ;[1 1 1] Reset function
  (`KismetSystemLibrary.K2_ClearAndInvalidateTimerHandle` (`self.CooldownTimer`)))

(event `self.SpawnBox.OnComponentEndOverlap`
  (params (OverlappedComponent :type "PrimitiveComponent Object Reference") (OtherActor :type "Actor Object Reference") (OtherComp :type "PrimitiveComponent Object Reference") (OtherBodyIndex :type Integer))
  (set `self.CanPlayerSpawn` true))

(event `self.SpawnBox.OnComponentBeginOverlap`
  (params (OverlappedComponent :type "PrimitiveComponent Object Reference") (OtherActor :type "Actor Object Reference") (OtherComp :type "PrimitiveComponent Object Reference") (OtherBodyIndex :type Integer) (bFromSweep :type Boolean) (SweepResult :type "HitResult Structure (by ref)"))
  (set `self.CanPlayerSpawn` false))

(fn `BelongsToArea`
  (params (Area :type Integer))
  (returns (BelongsTo :type Boolean))
  (return false))

(fn `CanSpawn`
  (returns (Spawnable :type Boolean))
  (return (`self.CanPlayerSpawn`)))

(fn `GetSpawnPoint`
  (returns (SpawnPoint :type "Transform Structure"))
  (bind _returnvalue (`self.GetTransform`))
  (bind (_asprimitive_component _bsuccess) (cast `PrimitiveComponent` (`self.RootComponent`) :!pure true))
  (bind (_ascapsule_collision _bsuccess_2) (cast `CapsuleComponent` _asprimitive_component :!pure true))
  (if (and _bsuccess _bsuccess_2)
    (return (`KismetMathLibrary.MakeTransform` (`KismetMathLibrary.MakeVector` (.x (.location _returnvalue)) (.y (.location _returnvalue)) (- (.z (.location _returnvalue)) (`CapsuleComponent.CapsuleHalfHeight` _ascapsule_collision))) (.rotation _returnvalue)))
    (else
      (return (`self.GetTransform`)))))

(fn `IsVRSpawn`
  (returns (VRspawn :type Boolean))
  (return true))

(fn `UserConstructionScript`)