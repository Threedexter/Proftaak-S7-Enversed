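; Basic projectile actor that deals point damage to what it hits when its ProjectileMovement component stops.
; On stop, it applies the damage with its instigator's controller credited, then spawns an impact particle emitter and plays a sound at the hit location.
; Damage, damage type, effects and destruction delay come from variables, and the actor destroys itself after that delay.
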(event `self.ProjectileMovement.OnProjectileStop`
  (params (ImpactResult :type "HitResult Structure (by ref)"))
  (bind (_bblockinghit _binitialoverlap _time _location _impactpoint _normal _impactnormal _physmat _hitactor) (`GameplayStatics.BreakHitResult` ImpactResult))
  (`GameplayStatics.ApplyPointDamage` _hitactor (`self.Damage`) _normal ImpactResult (`self.GetInstigatorController`) self "/Script/Engine.DamageType")
  (`GameplayStatics.SpawnEmitterAtLocation` (`self.ParticleOnImpact`) _location)
  (`GameplayStatics.PlaySoundAtLocation` (`self.SoundOnImpact`) _location)
  (`KismetSystemLibrary.Delay` (`self.DestructionDelay`))
  (`self.K2_DestroyActor`))

(fn `UserConstructionScript`)