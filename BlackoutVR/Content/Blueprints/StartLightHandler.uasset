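; Start light handler actor that switches off three groups of spotlights in sequence, like a starting-light countdown.
; BeginPlay builds the three light arrays, waits briefly, then runs StartFade if InitFade is set.
; StartFade starts a looping timer on TurnOffLight, which hides the group matching ActiveGroupCount (group 1 first when counting from three) and decrements it.
; The timer clears itself once the count reaches zero.
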(event `self.ReceiveBeginPlay`
  (set `self.LightGroup 3` (`|MakeArray` (`self.SpotLight (C-3)`) (`self.SpotLight (L-3)`) (`self.SpotLight (R-3)`)))
  (set `self.LightGroup 2` (`|MakeArray` (`self.SpotLight4 (C-4)`) (`self.SpotLight8 (L-2)`) (`self.SpotLight9 (L-4)`) (`self.SpotLight1 (R-4)`) (`self.SpotLight2 (R-2)`) (`self.SpotLight3 (C-2)`)))
  (set `self.LightGroup 1` (`|MakeArray` (`self.SpotLight1 (C-5)`) (`self.SpotLight2 (C-1)`) (`self.SpotLight6 (L-5)`) (`self.SpotLight7 (L-1)`) (`self.SpotLight4 (R-5)`) (`self.SpotLight3 (R-1)`)))
  (`KismetSystemLibrary.Delay` 3.0)
  (if (`self.InitFade`)
    (`self.StartFade`)))

(fn `StartFade`
  (bind _returnvalue (`KismetSystemLibrary.K2_SetTimer` self "TurnOffLight" (`self.StartInterval`) true))
  (set `self.TimerHandle` _returnvalue))

(fn `TurnGroupOff`
  (params (LightArray :type "Array of SpotLightComponent Object Reference"))
  (for _array_element LightArray
    (`SceneComponent.SetVisibility` _array_element false false))
  (return))

(fn `TurnOffLight`
  (switch `int` (`self.ActiveGroupCount`)
    (:`0`
      (`KismetSystemLibrary.K2_ClearAndInvalidateTimerHandle` (`self.TimerHandle`)))
    (:`1`
      (`self.TurnGroupOff` (`self.LightGroup 3`))
      (`/Engine/EditorBlueprintResources/StandardMacros.DecrementInt` (`self.ActiveGroupCount`) :!label _label))
    (:`2`
      (`self.TurnGroupOff` (`self.LightGroup 2`))
      (goto _label))
    (:`3`
      (`self.TurnGroupOff` (`self.LightGroup 1`))
      (goto _label))))

(fn `UserConstructionScript`)