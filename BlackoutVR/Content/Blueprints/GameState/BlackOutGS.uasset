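; BlackOutGS is a game state that starts and times a match for VR players and a spectator.
; Readying either role checks every PlayerState and the spectator flag, then starts the game once all are ready.
; Starting messages the game mode, sets a timer for GameTime that triggers the stop message, caches ScoreKeeper interface actors and calls CallInitGame.
; Start, stop and score setup route through Server-named events.
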(event `/Game/Blueprints/GameState/Interfaces/IBlackoutGameState.StartGame`
  ;[1 1 1] Starts the game timer
  (`self.StartGameServer`))

(event `StartGameServer`
  ;[1 1 1] Starts the game timer
  (message `/Game/Blueprints/GameMode/Interfaces/IBlackoutGM.StartGame` (`GameplayStatics.GetGameMode`) (`self.Players`))
  (bind _returnvalue (`KismetSystemLibrary.K2_SetTimerDelegate` (delegate `/Game/Blueprints/GameState/Interfaces/IBlackoutGameState.StopGame`) (`self.GameTime`)))
  (set `self.GameTimer` _returnvalue)
  (`self.InitScores`)
  (`self.InitGame`))

(event `/Game/Blueprints/GameState/Interfaces/IBlackoutGameState.StopGame`
  ;[1 1 1] Stops the game
  (`self.StopGameServer`))

(event `StopGameServer`
  ;[1 1 1] Stops the game
  (message `/Game/Blueprints/GameMode/Interfaces/IBlackoutGM.StopGame` (`GameplayStatics.GetGameMode`)))

(event `InitScoresClient`
  ;[1 1 1] Basic init
  (bind _outactors (`GameplayStatics.GetAllActorsWithInterface` "/Script/BlackoutVR.ScoreKeeper"))
  (set `self.ScoreActors` _outactors))

(event `InitScoresServer`
  ;[1 1 1] Basic init
  (`self.InitScoresClient`))

(event `/Game/Blueprints/GameState/Interfaces/IBlackoutGameState.InitScores`
  ;[1 1 1] Basic init
  (`self.InitScoresServer`))

(fn `ArePlayersReady`
  (returns (Ready :type Boolean))
  (bind _ready (`self.AreVRPlayersReady`))
  (bind _ready_2 (`/Game/Blueprints/GameState/Interfaces/IBlackoutGameState.AreSpectatorsReady`))
  (return (and _ready_2 _ready)))

(fn `AreSpectatorsReady`
  (returns (Ready :type Boolean))
  (return (`self.SpectatorReady`)))

(fn `AreVRPlayersReady`
  (returns (Ready :type Boolean))
  (locals (VRPlayersReady :type Boolean))
  (set `local.VRPlayersReady` true)
  (for _array_element (`self.PlayerArray`)
    (bind _ready (message `/Game/Blueprints/PlayerState/Interfaces/IPlayerState.IsReady` _array_element))
    (if (not _ready)
      (set `local.VRPlayersReady` false)
      (break)))
  (return (`local.VRPlayersReady`)))

(fn `GetGameTimer`
  (returns (Time :type "Float (double-precision)") (Timer :type "TimerHandle Structure"))
  (return (`self.GameTime`) (`self.GameTimer`)))

(fn `ReadySpectator`
  (params (Players :type "Array of Integer (by ref)") (ReadyState :type Boolean))
  (returns (Ready :type Boolean))
  (set `self.Players` Players)
  (set `self.SpectatorReady` ReadyState)
  (bind _ready (`self.ArePlayersReady`))
  (if _ready
    (`/Game/Blueprints/GameState/Interfaces/IBlackoutGameState.StartGame`)
    (return true)
    (else
      (return false))))

(fn `ReadyVRPlayer`
  (params (Controller :type "Controller Object Reference") (ReadyState :type Boolean))
  (returns (Ready :type Boolean))
  (bind _playerstate (`Controller.PlayerState` Controller))
  (`/Engine/EditorBlueprintResources/StandardMacros.IsValid` _playerstate
    (:`Is Valid`
      (bind _isready (message `/Game/Blueprints/PlayerState/Interfaces/IPlayerState.SetReadyState` _playerstate ReadyState))
      (if _isready
        (bind _ready (`self.ArePlayersReady`))
        (if _ready
          (`/Game/Blueprints/GameState/Interfaces/IBlackoutGameState.StartGame`)
          (return true)
          (else
            (return false)))
        (else
          _)))
    (:`Is Not Valid`
      _))
  (return false))

(fn `UserConstructionScript`)